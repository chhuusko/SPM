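; BP_Button is a crane control button that rotates one of three referenced cranes when activated.
; Its ActivateButton event branches on ButtonValue and calls RotateCrane on Crane1, Crane2 or Crane3 to match.
; Any other value does nothing, and the construction script is empty.
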(event Custom|ActivateButton
  (if (== (Variables|Default|GetButtonValue) 1)
    (Default|RotateCrane (Variables|Default|GetCrane1))
    (elif (== (Variables|Default|GetButtonValue) 2)
      (Default|RotateCrane (Variables|Default|GetCrane2))
      (elif (== (Variables|Default|GetButtonValue) 3)
        (Default|RotateCrane (Variables|Default|GetCrane3))))))

(fn ConstructionScript)