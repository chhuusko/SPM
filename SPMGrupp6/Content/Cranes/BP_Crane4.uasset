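; Crane actor that swings its pivot between two fixed yaw angles, carrying a container, button and jump pad.
; On BeginPlay it attaches those three child components to the pivot, keeping their world transforms.
; Each RotateCrane call alternately plays or reverses a timeline that interpolates the yaw, with a rotation sound.
; A DoOnce ignores further calls until the timeline finishes, which also fades the sound out.
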(event Custom|RotateCrane
  (Utilities|FlowControl|DoOnce false :!label _label
    (:Completed
      (Utilities|FlowControl|FlipFlop
        (:A
          (Audio|Components|Audio|Play (Variables|Default|GetRotation) 0.0)
          (bind _newtrack_1 (Timeline|Timeline Play)
            (:Update
              (Transformation|SetWorldRotation (Variables|Default|GetPivot) (Math|Rotator|MakeRotator 0.0 0.0 (.z (Math|Vector|Lerp(Vector) "0.000000,0.000000,-84.608999" "0.000000,0.000000,-40.000000" _newtrack_1))) false false))
            (:Finished
              (Audio|Components|Audio|FadeOut (Variables|Default|GetRotation) 1.0 0.0 "Linear" :!class /Script/Engine.AudioComponent)
              (goto _label Reset))))
        (:B
          (Audio|Components|Audio|Play (Variables|Default|GetRotation) 0.0)
          (Timeline|Timeline Reverse))))))

(event EventBeginPlay
  (CallFunction|AttachingActorstoCrane))

(fn ConstructionScript)

(fn AttachingActorstoCrane
  (Transformation|AttachComponentToComponent (Variables|Default|GetContainerChild) (Variables|Default|GetPivot) "None" "KeepWorld" "KeepWorld" "KeepWorld" true)
  (Transformation|AttachComponentToComponent (Variables|Default|GetButtonChild) (Variables|Default|GetPivot) "None" "KeepWorld" "KeepWorld" "KeepWorld" true)
  (Transformation|AttachComponentToComponent (Variables|Default|GetJumpPadChild) (Variables|Default|GetPivot) "None" "KeepWorld" "KeepWorld" "KeepWorld" true))