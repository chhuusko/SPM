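; A crane actor that swings its load between two fixed yaw angles each time RotateCrane is called.
; On BeginPlay it attaches the container, box, magnet parts and button to Pivot, keeping world transforms so they turn with it.
; RotateCrane alternates playing and reversing a Timeline that sets Pivot's world yaw, with a DoOnce blocking new calls until the swing finishes.
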(event Custom|RotateCrane
  (Utilities|FlowControl|DoOnce false :!label _label
    (:Completed
      (Utilities|FlowControl|FlipFlop
        (:A
          (bind _newtrack_1 (Timeline|Timeline Play)
            (:Update
              (Transformation|SetWorldRotation (Variables|Default|GetPivot) (Math|Rotator|MakeRotator 0.0 0.0 (.z (Math|Vector|Lerp(Vector) "0.000000,0.000000,22.164705" "0.000000,0.000000,-47.835294" _newtrack_1))) false false))
            (:Finished
              (goto _label Reset))))
        (:B
          (Timeline|Timeline Reverse))))))

(event EventBeginPlay
  (CallFunction|AttachingActorstoCrane))

(fn ConstructionScript)

(fn AttachingActorstoCrane
  (Transformation|AttachComponentToComponent (Variables|Default|GetContainerChild) (Variables|Default|GetPivot) "None" "KeepWorld" "KeepWorld" "KeepWorld" true)
  (Transformation|AttachComponentToComponent (Variables|Default|GetBoxChild) (Variables|Default|GetPivot) "None" "KeepWorld" "KeepWorld" "KeepWorld" true)
  (Transformation|AttachComponentToComponent (Variables|Default|GetMagnetChild1) (Variables|Default|GetPivot) "None" "KeepWorld" "KeepWorld" "KeepWorld" true)
  (Transformation|AttachComponentToComponent (Variables|Default|GetMagnetChild2) (Variables|Default|GetPivot) "None" "KeepWorld" "KeepWorld" "KeepWorld" true)
  (Transformation|AttachComponentToComponent (Variables|Default|GetMagnetChild3) (Variables|Default|GetPivot) "None" "KeepWorld" "KeepWorld" "KeepWorld" true)
  (Transformation|AttachComponentToComponent (Variables|Default|GetMagnetChild4) (Variables|Default|GetPivot) "None" "KeepWorld" "KeepWorld" "KeepWorld" true)
  (Transformation|AttachComponentToComponent (Variables|Default|GetMagnetArmChild1) (Variables|Default|GetPivot) "None" "KeepWorld" "KeepWorld" "KeepWorld" true)
  (Transformation|AttachComponentToComponent (Variables|Default|GetMagnetArmChild2) (Variables|Default|GetPivot) "None" "KeepWorld" "KeepWorld" "KeepWorld" true)
  (Transformation|AttachComponentToComponent (Variables|Default|GetMagnetBottomChild1) (Variables|Default|GetPivot) "None" "KeepWorld" "KeepWorld" "KeepWorld" true)
  (Transformation|AttachComponentToComponent (Variables|Default|GetMagnetBottomChild2) (Variables|Default|GetPivot) "None" "KeepWorld" "KeepWorld" "KeepWorld" true)
  (Transformation|AttachComponentToComponent (Variables|Default|GetButtonChild) (Variables|Default|GetPivot) "None" "KeepWorld" "KeepWorld" "KeepWorld" true))