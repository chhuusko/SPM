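; Shooter character Blueprint that lets the player switch between a first-person camera and a second camera.
; The IA_SwitchPerspective Enhanced Input action drives a FlipFlop that activates one camera component and deactivates the other.
; The first press activates the Camera component, and each later press alternates between the two.
; BeginPlay is empty, and the Tick and overlap events are disabled.
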(event Input|EnhancedActionEvents|EnhancedInputActionIA_SwitchPerspective
  (params (ActionValue :type Boolean) (ElapsedSeconds :type Float%20%28double-precision%29) (TriggeredSeconds :type Float%20%28double-precision%29) (InputAction :type Input%20Action%20Object%20Reference :default "/Game/Inputs/IA_SwitchPerspective.IA_SwitchPerspective"))
  (:Started
    (Utilities|FlowControl|FlipFlop
      (:A
        (Components|Activation|SetActive (Variables|Default|GetFirstPersonCamera) false false)
        (Components|Activation|SetActive (Variables|Default|GetCamera) true false))
      (:B
        (Components|Activation|SetActive (Variables|Default|GetCamera) false false)
        (Components|Activation|SetActive (Variables|Default|GetFirstPersonCamera) true false)))))

(event EventBeginPlay)

(event Collision|EventActorBeginOverlap
  (params (OtherActor :type Actor%20Object%20Reference))
  (|CallParentFunction OtherActor) ; This node is disabled and will not be called.\nDrag off pins to build functionality.
)

(event EventTick
  (params (DeltaSeconds :type Float%20%28single-precision%29))
  (|CallParentFunction DeltaSeconds) ; This node is disabled and will not be called.\nDrag off pins to build functionality.
)

(fn ConstructionScript
  (|CallParentFunction))