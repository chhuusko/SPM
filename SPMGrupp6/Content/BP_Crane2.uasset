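; Crane Blueprint that swings its Pivot between two fixed yaw angles each time RotateCrane is triggered.
; On BeginPlay it attaches the container and button children to the Pivot, keeping world transforms so they turn with it.
; A FlipFlop alternately plays and reverses a Timeline that interpolates the yaw, while a DoOnce blocks retriggering until the Timeline finishes.
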(event Custom|RotateCrane
  (Utilities|FlowControl|DoOnce false :!label _label
    (:Completed
      (Utilities|FlowControl|FlipFlop
        (:A
          (bind _newtrack_1 (Timeline|Timeline Play)
            (:Update
              (Transformation|SetWorldRotation (Variables|Default|GetPivot) (Math|Rotator|MakeRotator 0.0 0.0 (.z (Math|Vector|Lerp(Vector) "0.000000,0.000000,10.391000" "0.000000,0.000000,-25.000000" _newtrack_1))) false false))
            (:Finished
              (goto _label Reset))))
        (:B
          (Timeline|Timeline Reverse))))))

(event EventBeginPlay
  (CallFunction|AttachingActorstoCrane))

(fn ConstructionScript)

(fn AttachingActorstoCrane
  (Transformation|AttachComponentToComponent (Variables|Default|GetContainerChild) (Variables|Default|GetPivot) "None" "KeepWorld" "KeepWorld" "KeepWorld" true)
  (Transformation|AttachComponentToComponent (Variables|Default|GetButtonChild) (Variables|Default|GetPivot) "None" "KeepWorld" "KeepWorld" "KeepWorld" true))