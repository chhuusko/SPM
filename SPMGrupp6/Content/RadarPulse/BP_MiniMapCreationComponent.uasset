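; Actor component that gives each local perspective-shooter player a minimap with a radar pulse, supporting two players.
; Player controller ID selects the widget class and the render target for the owner's SceneCapture2D.
; Tick retries widget creation and texture assignment until both succeed, and applies flagged map size changes as ortho width.
; It also reads pulse cooldown progress from the widget and pushes tracking distance and cooldown when flagged.
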(event EventBeginPlay
  (CallFunction|CreateMiniMap))

(event EventTick
  (params (DeltaSeconds :type Float%20%28single-precision%29))
  (CallFunction|UpdateMap)
  (|UpdatePulse))

(fn CreateMiniMap
  (bind (_player _id _success) (CallFunction|GetPlayerID))
  (if _success
    (if (== _id 0)
      (Variables|Default|SetWidgetClass "/Game/RadarPulse/WBP_MiniMap_1.WBP_MiniMap_1_C")
      (else
        (Variables|Default|SetWidgetClass "/Game/RadarPulse/WBP_MiniMap_2.WBP_MiniMap_2_C")))
    (bind _returnvalue (UserInterface|CreateWidget (Variables|Default|GetWidgetClass) _player))
    (bind _output_get (Variables|Default|SetCreatedWidget _returnvalue))
    (bind _returnvalue_2 (UserInterface|Viewport|AddtoPlayerScreen _output_get))
    (bind _output_get_2 (Variables|Default|SetCreated _returnvalue_2))
    (Development|PrintString (Utilities|String|Append "Created (" (Utilities|String|ToString(Boolean) _output_get_2) ") widget for player: " (Utilities|String|ToString(Integer) _id)) (Variables|Default|GetPrintDebugToScreen))))

(fn GetPlayerID
  (bind _asbp_perspective_shooter_character (Utilities|Casting|CastToBP_PerspectiveShooterCharacter (Components|GetOwner))
    (:then
      (if (!= -1 (Class|GameplayStatics|GetPlayerControllerID (Pawn|GetLocalViewingPlayerController _asbp_perspective_shooter_character)))
        _
        (else
          _)))
    (:CastFailed
      _))
  (return (Pawn|GetLocalViewingPlayerController _asbp_perspective_shooter_character) (Class|GameplayStatics|GetPlayerControllerID (Pawn|GetLocalViewingPlayerController _asbp_perspective_shooter_character)) (!= -1 (Class|GameplayStatics|GetPlayerControllerID (Pawn|GetLocalViewingPlayerController _asbp_perspective_shooter_character)))))

(fn SetMiniMapTexture
  (bind _returnvalue (Components|GetOwner))
  (bind _returnvalue_2 (Actor|GetComponentbyClass _returnvalue "/Script/Engine.SceneCaptureComponent2D"))
  (bind (_player _id _success) (CallFunction|GetPlayerID))
  (if _success
    (if (== _id 0)
      (Variables|/Script/Engine.SceneCaptureComponent2D|SetTextureTarget _returnvalue_2 "/Game/RadarPulse/RT_MiniMap_1.RT_MiniMap_1")
      (else
        (Variables|/Script/Engine.SceneCaptureComponent2D|SetTextureTarget _returnvalue_2 "/Game/RadarPulse/RT_MiniMap_2.RT_MiniMap_2")))
    (Variables|Default|SetTextureSet true)))

(fn UpdateMap
  (if (Variables|Default|GetCreated)
    (if (Variables|Default|GetTextureSet)
      (if (Variables|Default|GetUpdateMiniMapSize)
        (Variables|/Script/Engine.SceneCaptureComponent2D|SetOrthoWidth (Actor|GetComponentbyClass (Components|GetOwner) "/Script/Engine.SceneCaptureComponent2D") (Variables|Default|GetMiniMapSize) :!label _label)
        (Variables|Default|SetUpdateMiniMapSize false))
      (else
        (CallFunction|SetMiniMapTexture)
        (goto _label)))
    (else
      (CallFunction|CreateMiniMap))))

(fn UpdatePulseValuesFunc
  (Variables|/Game/RadarPulse/WBP_MiniMap_Base.WBP_MiniMap_Base_C|SetTrackingDistance (Variables|Default|GetCreatedWidget) (Variables|Default|GetTrackingDistance))
  (Variables|/Game/RadarPulse/WBP_MiniMap_Base.WBP_MiniMap_Base_C|SetPulseCooldown (Variables|Default|GetCreatedWidget) (Variables|Default|GetPulseCooldown)))