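; Tutorial manager that walks the player through movement, combat and weapon lessons as an ordered series of on-screen prompts.
; ProgressTutorial switches on TutorialStep to create that step's prompt widget, ending with a completion prompt.
; Player-action events are gated by step and DoOnce, then complete the prompt, wait, remove it and advance.
; Weapon swapping requires both scroll and hotswap; the third drone step auto-completes given enough character resources.
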(event Custom|ProgressTutorial
  (switch int (Variables|Default|GetTutorialStep)
    (:Default
      (bind _returnvalue (UserInterface|CreateWidget "/Game/TutorialLevel/WBP_TutorialCompletePrompt.WBP_TutorialCompletePrompt_C"))
      (Variables|Default|SetTutorialCompleteWidget _returnvalue)
      (UserInterface|Viewport|AddtoPlayerScreen _returnvalue))
    (:0
      (bind _returnvalue_2 (UserInterface|CreateWidget "/Game/TutorialLevel/WBP_MovePrompt.WBP_MovePrompt_C"))
      (Variables|Default|SetMoveWidget _returnvalue_2)
      (UserInterface|Viewport|AddtoPlayerScreen _returnvalue_2))
    (:1
      (bind _returnvalue_3 (UserInterface|CreateWidget "/Game/TutorialLevel/WBP_SprintPrompt.WBP_SprintPrompt_C"))
      (Variables|Default|SetSprintWidget _returnvalue_3)
      (UserInterface|Viewport|AddtoPlayerScreen _returnvalue_3))
    (:2
      (bind _returnvalue_4 (UserInterface|CreateWidget "/Game/TutorialLevel/WBP_JumpPrompt.WBP_JumpPrompt_C"))
      (Variables|Default|SetJumpWidget _returnvalue_4)
      (UserInterface|Viewport|AddtoPlayerScreen _returnvalue_4))
    (:3
      (bind _returnvalue_5 (UserInterface|CreateWidget "/Game/TutorialLevel/WBP_JetpackPrompt.WBP_JetpackPrompt_C"))
      (Variables|Default|SetJetpackWidget _returnvalue_5)
      (UserInterface|Viewport|AddtoPlayerScreen _returnvalue_5))
    (:4
      (bind _returnvalue_6 (UserInterface|CreateWidget "/Game/TutorialLevel/WBP_DashPrompt.WBP_DashPrompt_C"))
      (Variables|Default|SetDashWidget _returnvalue_6)
      (UserInterface|Viewport|AddtoPlayerScreen _returnvalue_6))
    (:5
      (bind _returnvalue_7 (UserInterface|CreateWidget "/Game/TutorialLevel/WBP_JumppadPrompt.WBP_JumppadPrompt_C"))
      (Variables|Default|SetJumppadWidget _returnvalue_7)
      (UserInterface|Viewport|AddtoPlayerScreen _returnvalue_7))
    (:6
      (bind _returnvalue_8 (UserInterface|CreateWidget "/Game/TutorialLevel/WBP_MovementChallengePrompt.WBP_MovementChallengePrompt_C"))
      (Variables|Default|SetMovementChallengeWidget _returnvalue_8)
      (UserInterface|Viewport|AddtoPlayerScreen _returnvalue_8))
    (:7
      (bind _returnvalue_9 (UserInterface|CreateWidget "/Game/TutorialLevel/WBP_FireWeaponPrompt.WBP_FireWeaponPrompt_C"))
      (Variables|Default|SetFireWeaponWidget _returnvalue_9)
      (UserInterface|Viewport|AddtoPlayerScreen _returnvalue_9))
    (:8
      (bind _returnvalue_10 (UserInterface|CreateWidget "/Game/TutorialLevel/WBP_ReloadPrompt.WBP_ReloadPrompt_C"))
      (Variables|Default|SetReloadWeaponWidget _returnvalue_10)
      (UserInterface|Viewport|AddtoPlayerScreen _returnvalue_10))
    (:9
      (bind _returnvalue_11 (UserInterface|CreateWidget "/Game/TutorialLevel/WBP_KillDronePrompt.WBP_KillDronePrompt_C"))
      (Variables|Default|SetKillDroneWidget _returnvalue_11)
      (UserInterface|Viewport|AddtoPlayerScreen _returnvalue_11))
    (:10
      (bind _returnvalue_12 (UserInterface|CreateWidget "/Game/TutorialLevel/WBP_KillDrone2Prompt.WBP_KillDrone2Prompt_C"))
      (Variables|Default|SetKillDrone2Widget _returnvalue_12)
      (UserInterface|Viewport|AddtoPlayerScreen _returnvalue_12))
    (:11
      (bind _returnvalue_13 (UserInterface|CreateWidget "/Game/TutorialLevel/WBP_UnlockWeaponPrompt.WBP_UnlockWeaponPrompt_C"))
      (Variables|Default|SetUnlockWeaponWidget _returnvalue_13)
      (UserInterface|Viewport|AddtoPlayerScreen _returnvalue_13))
    (:12
      (bind _returnvalue_14 (UserInterface|CreateWidget "/Game/TutorialLevel/WBP_SwapWeaponPrompt.WBP_SwapWeaponPrompt_C"))
      (Variables|Default|SetSwapWeaponWidget _returnvalue_14)
      (UserInterface|Viewport|AddtoPlayerScreen _returnvalue_14))
    (:13
      (bind _returnvalue_15 (UserInterface|CreateWidget "/Game/TutorialLevel/WBP_KillDrone3Prompt.WBP_KillDrone3Prompt_C"))
      (Variables|Default|SetKillDrone3Widget _returnvalue_15)
      (UserInterface|Viewport|AddtoPlayerScreen _returnvalue_15)
      (bind _returnvalue_16 (Actor|GetActorOfClass "/Game/BP_PerspectiveShooterCharacter.BP_PerspectiveShooterCharacter_C"))
      (bind _asbp_perspective_shooter_character (Utilities|Casting|CastToBP_PerspectiveShooterCharacter _returnvalue_16))
      (bind _returnvalue_17 (Class|Resources|GetResourceAmount (Variables|/Game/BP_PerspectiveShooterCharacter.BP_PerspectiveShooterCharacter_C|GetResources _asbp_perspective_shooter_character)))
      (if (>= _returnvalue_17 4)
        (CallFunction|PlayerKilledDrone3)))
    (:14
      (bind _returnvalue_18 (UserInterface|CreateWidget "/Game/TutorialLevel/WBP_UpgradeWeaponPrompt.WBP_UpgradeWeaponPrompt_C"))
      (Variables|Default|SetUpgradeWeaponWidget _returnvalue_18)
      (UserInterface|Viewport|AddtoPlayerScreen _returnvalue_18))
    (:15
      (bind _returnvalue_19 (UserInterface|CreateWidget "/Game/TutorialLevel/WBP_AltFirePrompt.WBP_AltFirePrompt_C"))
      (Variables|Default|SetAltFireWidget _returnvalue_19)
      (UserInterface|Viewport|AddtoPlayerScreen _returnvalue_19))))

(event Custom|PlayerHotswapped
  (if (== (Variables|Default|GetTutorialStep) 12)
    (Variables|Default|SetHotswapDone true)
    (if (and (Variables|Default|GetHotswapDone) (Variables|Default|GetScrollSwapDone))
      (Utilities|FlowControl|DoOnce false
        (:Completed
          (Default|CompleteStep (Variables|Default|GetSwapWeaponWidget))
          (Utilities|FlowControl|Delay 3.0)
          (Variables|Default|SetTutorialStep 13)
          (Widget|RemovefromParent (Variables|Default|GetSwapWeaponWidget))
          (CallFunction|ProgressTutorial))))))

(event Custom|PlayerUpgradedWeapon
  (if (== (Variables|Default|GetTutorialStep) 14)
    (Utilities|FlowControl|DoOnce false
      (:Completed
        (Default|CompleteStep (Variables|Default|GetUpgradeWeaponWidget))
        (Utilities|FlowControl|Delay 3.0)
        (Variables|Default|SetTutorialStep 15)
        (Widget|RemovefromParent (Variables|Default|GetUpgradeWeaponWidget))
        (CallFunction|ProgressTutorial)))))

(event Custom|PlayerUsedJetpack
  (if (== (Variables|Default|GetTutorialStep) 3)
    (Utilities|FlowControl|DoOnce false
      (:Completed
        (Default|CompleteStep (Variables|Default|GetJetpackWidget))
        (Utilities|FlowControl|Delay 3.0)
        (Variables|Default|SetTutorialStep 4)
        (Widget|RemovefromParent (Variables|Default|GetJetpackWidget))
        (CallFunction|ProgressTutorial)))))

(event Custom|PlayerJumped
  (if (== (Variables|Default|GetTutorialStep) 2)
    (Utilities|FlowControl|DoOnce false
      (:Completed
        (Default|CompleteStep (Variables|Default|GetJumpWidget))
        (Utilities|FlowControl|Delay 3.0)
        (Variables|Default|SetTutorialStep 3)
        (Widget|RemovefromParent (Variables|Default|GetJumpWidget))
        (CallFunction|ProgressTutorial)))))

(event Custom|PlayerUsedDash
  (if (== (Variables|Default|GetTutorialStep) 4)
    (Utilities|FlowControl|DoOnce false
      (:Completed
        (Default|CompleteStep (Variables|Default|GetDashWidget))
        (Utilities|FlowControl|Delay 3.0)
        (Variables|Default|SetTutorialStep 5)
        (Widget|RemovefromParent (Variables|Default|GetDashWidget))
        (CallFunction|ProgressTutorial)))))

(event Custom|PlayerUnlockedWeapon
  (if (== (Variables|Default|GetTutorialStep) 11)
    (Utilities|FlowControl|DoOnce false
      (:Completed
        (Default|CompleteStep (Variables|Default|GetUnlockWeaponWidget))
        (Utilities|FlowControl|Delay 3.0)
        (Variables|Default|SetTutorialStep 12)
        (Widget|RemovefromParent (Variables|Default|GetUnlockWeaponWidget))
        (CallFunction|ProgressTutorial)))))

(event Custom|MovementChallengeDone
  (if (== (Variables|Default|GetTutorialStep) 6)
    (Utilities|FlowControl|DoOnce false
      (:Completed
        (Default|CompleteStep (Variables|Default|GetMovementChallengeWidget))
        (Utilities|FlowControl|Delay 3.0)
        (Variables|Default|SetTutorialStep 7)
        (Widget|RemovefromParent (Variables|Default|GetMovementChallengeWidget))
        (CallFunction|ProgressTutorial)))))

(event Custom|PlayerSprinted
  (if (== (Variables|Default|GetTutorialStep) 1)
    (Utilities|FlowControl|DoOnce false
      (:Completed
        (Default|CompleteStep (Variables|Default|GetSprintWidget))
        (Utilities|FlowControl|Delay 3.0)
        (Variables|Default|SetTutorialStep 2)
        (Widget|RemovefromParent (Variables|Default|GetSprintWidget))
        (CallFunction|ProgressTutorial)))))

(event Custom|PlayerUsedJumppad
  (if (== (Variables|Default|GetTutorialStep) 5)
    (Utilities|FlowControl|DoOnce false
      (:Completed
        (Default|CompleteStep (Variables|Default|GetJumppadWidget))
        (Utilities|FlowControl|Delay 3.0)
        (Variables|Default|SetTutorialStep 6)
        (Widget|RemovefromParent (Variables|Default|GetJumppadWidget))
        (CallFunction|ProgressTutorial)))))

(event Custom|PlayerMoved
  (if (== (Variables|Default|GetTutorialStep) 0)
    (Utilities|FlowControl|DoOnce false
      (:Completed
        (Default|CompleteStep (Variables|Default|GetMoveWidget))
        (Utilities|FlowControl|Delay 3.0)
        (Variables|Default|SetTutorialStep 1)
        (Widget|RemovefromParent (Variables|Default|GetMoveWidget))
        (CallFunction|ProgressTutorial)))))

(event Custom|PlayerKilledDrone3
  (if (== (Variables|Default|GetTutorialStep) 13)
    (Utilities|FlowControl|DoOnce false
      (:Completed
        (Default|CompleteStep (Variables|Default|GetKillDrone3Widget))
        (Utilities|FlowControl|Delay 3.0)
        (Variables|Default|SetTutorialStep 14)
        (Widget|RemovefromParent (Variables|Default|GetKillDrone3Widget))
        (CallFunction|ProgressTutorial)))))

(event Custom|PlayerKilledDrone2
  (if (== (Variables|Default|GetTutorialStep) 10)
    (Utilities|FlowControl|DoOnce false
      (:Completed
        (Default|CompleteStep (Variables|Default|GetKillDrone2Widget))
        (Utilities|FlowControl|Delay 3.0)
        (Variables|Default|SetTutorialStep 11)
        (Widget|RemovefromParent (Variables|Default|GetKillDrone2Widget))
        (CallFunction|ProgressTutorial)))))

(event Custom|PlayerUsedAltFire
  (if (== (Variables|Default|GetTutorialStep) 15)
    (Utilities|FlowControl|DoOnce false
      (:Completed
        (Default|CompleteStep (Variables|Default|GetAltFireWidget))
        (Utilities|FlowControl|Delay 3.0)
        (Variables|Default|SetTutorialStep 16)
        (Widget|RemovefromParent (Variables|Default|GetAltFireWidget))
        (CallFunction|ProgressTutorial)))))

(event Custom|PlayerFiredWeapon
  (if (== (Variables|Default|GetTutorialStep) 7)
    (Utilities|FlowControl|DoOnce false
      (:Completed
        (Default|CompleteStep (Variables|Default|GetFireWeaponWidget))
        (Utilities|FlowControl|Delay 3.0)
        (Variables|Default|SetTutorialStep 8)
        (Widget|RemovefromParent (Variables|Default|GetFireWeaponWidget))
        (CallFunction|ProgressTutorial)))))

(event Custom|PlayerSwappedWeapon
  (if (== (Variables|Default|GetTutorialStep) 12)
    (Variables|Default|SetScrollSwapDone true)
    (if (and (Variables|Default|GetHotswapDone) (Variables|Default|GetScrollSwapDone))
      (Utilities|FlowControl|DoOnce false
        (:Completed
          (Default|CompleteStep (Variables|Default|GetSwapWeaponWidget))
          (Utilities|FlowControl|Delay 3.0)
          (Variables|Default|SetTutorialStep 13)
          (Widget|RemovefromParent (Variables|Default|GetSwapWeaponWidget))
          (CallFunction|ProgressTutorial))))))

(event Custom|PlayerReloaded
  (if (== (Variables|Default|GetTutorialStep) 8)
    (Utilities|FlowControl|DoOnce false
      (:Completed
        (Default|CompleteStep (Variables|Default|GetReloadWeaponWidget))
        (Utilities|FlowControl|Delay 3.0)
        (Variables|Default|SetTutorialStep 9)
        (Widget|RemovefromParent (Variables|Default|GetReloadWeaponWidget))
        (CallFunction|ProgressTutorial)))))

(event Custom|PlayerKilledDrone
  (if (== (Variables|Default|GetTutorialStep) 9)
    (Utilities|FlowControl|DoOnce false
      (:Completed
        (Default|CompleteStep (Variables|Default|GetKillDroneWidget))
        (Utilities|FlowControl|Delay 3.0)
        (Variables|Default|SetTutorialStep 10)
        (Widget|RemovefromParent (Variables|Default|GetKillDroneWidget))
        (CallFunction|ProgressTutorial)))))

(fn ConstructionScript)