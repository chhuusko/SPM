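; BP_InvisibleWall1 is an invisible wall in the tutorial map that moves from its starting position by a set offset when triggered.
; It caches the Box component's world location on BeginPlay.
; The MoveWall event passes through a DoOnce, then plays a timeline that lerps the box toward start plus MovementOffset without sweeping.
; Nothing in this Blueprint calls MoveWall or resets it, so the move happens only once.
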(event Custom|MoveWall
  (Utilities|FlowControl|DoOnce false
    (:Completed
      (bind _newtrack_0 (Timeline|Timeline_0 Play)
        (:Update
          (Transformation|SetWorldLocation (Variables|Default|GetBox) (Math|Vector|Lerp(Vector) (Variables|Default|GetStartingLocation) (+ (Variables|Default|GetStartingLocation) (Variables|Default|GetMovementOffset)) _newtrack_0) false false))))))

(event EventBeginPlay
  (Variables|Default|SetStartingLocation (Transformation|GetWorldLocation (Variables|Default|GetBox))))

(fn ConstructionScript)