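; Tutorial component on the player character that walks each of two players through ordered prompts for movement, combat, drone kills and weapon upgrades.
; ProgressTutorial creates the current step's widget on that player's screen, indexed by whether the owner is the first character.
; Player action events complete their matching step once, play a stinger, then advance after a delay.
; Drone kill steps auto-complete when resources already suffice; weapon swapping needs both scroll and hotswap.
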(event Custom|ProgressTutorial
  (params (OwningPlayer :type Player%20Controller%20Object%20Reference))
  (bind _playerindex (Variables|Default|GetPlayerIndex))
  (bind _returnvalue (Game|GetPlayerController _playerindex))
  (CallFunction|SetPlayerIndex)
  (switch int (Variables|Default|GetTutorialStep)
    (:Default
      (bind _returnvalue_2 (UserInterface|CreateWidget "/Game/TutorialMap/WBP_TutorialCompletePrompt.WBP_TutorialCompletePrompt_C" _returnvalue))
      (Variables|Default|SetTutorialCompleteWidget _returnvalue_2)
      (UserInterface|Viewport|AddtoPlayerScreen _returnvalue_2))
    (:0
      (bind _returnvalue_3 (UserInterface|CreateWidget "/Game/TutorialMap/WBP_MovePrompt.WBP_MovePrompt_C" _returnvalue))
      (Variables|Default|SetMoveWidget _returnvalue_3)
      (UserInterface|Viewport|AddtoPlayerScreen _returnvalue_3))
    (:1
      (bind _returnvalue_4 (UserInterface|CreateWidget "/Game/TutorialMap/WBP_FireWeaponPrompt.WBP_FireWeaponPrompt_C" _returnvalue))
      (Variables|Default|SetFireWeaponWidget _returnvalue_4)
      (UserInterface|Viewport|AddtoPlayerScreen _returnvalue_4))
    (:2
      (bind _returnvalue_5 (UserInterface|CreateWidget "/Game/TutorialMap/WBP_ReloadPrompt.WBP_ReloadPrompt_C" _returnvalue))
      (Variables|Default|SetReloadWeaponWidget _returnvalue_5)
      (UserInterface|Viewport|AddtoPlayerScreen _returnvalue_5))
    (:3
      (bind _returnvalue_6 (UserInterface|CreateWidget "/Game/TutorialMap/WBP_SprintPrompt.WBP_SprintPrompt_C" _returnvalue))
      (Variables|Default|SetSprintWidget _returnvalue_6)
      (UserInterface|Viewport|AddtoPlayerScreen _returnvalue_6))
    (:4
      (bind _returnvalue_7 (UserInterface|CreateWidget "/Game/TutorialMap/WBP_JumpPrompt.WBP_JumpPrompt_C" _returnvalue))
      (Variables|Default|SetJumpWidget _returnvalue_7)
      (UserInterface|Viewport|AddtoPlayerScreen _returnvalue_7))
    (:5
      (bind _returnvalue_8 (UserInterface|CreateWidget "/Game/TutorialMap/WBP_JetpackPrompt.WBP_JetpackPrompt_C" _returnvalue))
      (Variables|Default|SetJetpackWidget _returnvalue_8)
      (UserInterface|Viewport|AddtoPlayerScreen _returnvalue_8))
    (:6
      (bind _returnvalue_9 (UserInterface|CreateWidget "/Game/TutorialMap/WBP_DashPrompt.WBP_DashPrompt_C" _returnvalue))
      (Variables|Default|SetDashWidget _returnvalue_9)
      (UserInterface|Viewport|AddtoPlayerScreen _returnvalue_9))
    (:7
      (bind _returnvalue_10 (UserInterface|CreateWidget "/Game/TutorialMap/WBP_JumppadPrompt.WBP_JumppadPrompt_C" _returnvalue))
      (Variables|Default|SetJumppadWidget _returnvalue_10)
      (UserInterface|Viewport|AddtoPlayerScreen _returnvalue_10))
    (:8
      (bind _returnvalue_11 (UserInterface|CreateWidget "/Game/TutorialMap/WBP_MovementChallengePrompt.WBP_MovementChallengePrompt_C" _returnvalue))
      (Variables|Default|SetMovementChallengeWidget _returnvalue_11)
      (UserInterface|Viewport|AddtoPlayerScreen _returnvalue_11))
    (:9
      (bind _returnvalue_12 (UserInterface|CreateWidget "/Game/TutorialMap/WBP_KillDronePrompt.WBP_KillDronePrompt_C" _returnvalue))
      (Variables|Default|SetKillDroneWidget _returnvalue_12)
      (UserInterface|Viewport|AddtoPlayerScreen _returnvalue_12))
    (:10
      (bind _returnvalue_13 (UserInterface|CreateWidget "/Game/TutorialMap/WBP_KillDrone2Prompt.WBP_KillDrone2Prompt_C" _returnvalue))
      (Variables|Default|SetKillDrone2Widget _returnvalue_13)
      (UserInterface|Viewport|AddtoPlayerScreen _returnvalue_13)
      (bind _returnvalue_14 (Actor|GetActorOfClass "/Game/BP_PerspectiveShooterCharacter.BP_PerspectiveShooterCharacter_C"))
      (bind _returnvalue_15 (Class|Resources|GetResourceAmount (Variables|/Game/BP_PerspectiveShooterCharacter.BP_PerspectiveShooterCharacter_C|GetResources _returnvalue_14)))
      (if (>= _returnvalue_15 2)
        (bind _asbp_shooter_player_controller (Utilities|Casting|CastToBP_ShooterPlayerController (Pawn|GetController _returnvalue_14)))
        (CallFunction|PlayerKilledDrone2 _asbp_shooter_player_controller)))
    (:11
      (bind _returnvalue_16 (UserInterface|CreateWidget "/Game/TutorialMap/WBP_UnlockWeaponPrompt.WBP_UnlockWeaponPrompt_C" _returnvalue))
      (Variables|Default|SetUnlockWeaponWidget _returnvalue_16)
      (UserInterface|Viewport|AddtoPlayerScreen _returnvalue_16))
    (:12
      (bind _returnvalue_17 (UserInterface|CreateWidget "/Game/TutorialMap/WBP_SwapWeaponPrompt.WBP_SwapWeaponPrompt_C" _returnvalue))
      (Variables|Default|SetSwapWeaponWidget _returnvalue_17)
      (UserInterface|Viewport|AddtoPlayerScreen _returnvalue_17))
    (:13
      (bind _returnvalue_18 (UserInterface|CreateWidget "/Game/TutorialMap/WBP_KillDrone3Prompt.WBP_KillDrone3Prompt_C" _returnvalue))
      (Variables|Default|SetKillDrone3Widget _returnvalue_18)
      (UserInterface|Viewport|AddtoPlayerScreen _returnvalue_18)
      (bind _returnvalue_19 (Actor|GetActorOfClass "/Game/BP_PerspectiveShooterCharacter.BP_PerspectiveShooterCharacter_C"))
      (bind _returnvalue_20 (Class|Resources|GetResourceAmount (Variables|/Game/BP_PerspectiveShooterCharacter.BP_PerspectiveShooterCharacter_C|GetResources _returnvalue_19)))
      (if (>= _returnvalue_20 4)
        (bind _asbp_shooter_player_controller_2 (Utilities|Casting|CastToBP_ShooterPlayerController (Pawn|GetController _returnvalue_19)))
        (CallFunction|PlayerKilledDrone3 _asbp_shooter_player_controller_2)))
    (:14
      (bind _returnvalue_21 (UserInterface|CreateWidget "/Game/TutorialMap/WBP_UpgradeWeaponPrompt.WBP_UpgradeWeaponPrompt_C" _returnvalue))
      (Variables|Default|SetUpgradeWeaponWidget _returnvalue_21)
      (UserInterface|Viewport|AddtoPlayerScreen _returnvalue_21))
    (:15
      (bind _returnvalue_22 (UserInterface|CreateWidget "/Game/TutorialMap/WBP_AltFirePrompt.WBP_AltFirePrompt_C" _returnvalue))
      (Variables|Default|SetAltFireWidget _returnvalue_22)
      (UserInterface|Viewport|AddtoPlayerScreen _returnvalue_22))))

(event Custom|PlayerHotswapped
  (params (Owning%20Player :type Player%20Controller%20Object%20Reference))
  (if (== (Variables|Default|GetTutorialStep) 12)
    (Variables|Default|SetHotswapDone true)
    (if (and (Variables|Default|GetHotswapDone) (Variables|Default|GetScrollSwapDone))
      (Utilities|FlowControl|DoOnce false
        (:Completed
          (Default|CompleteStep (Variables|Default|GetSwapWeaponWidget))
          (Audio|SpawnSound2D "/Game/Audio/Stingers/stinger_complete.stinger_complete" 1.0 1.0 0.0 0)
          (Utilities|FlowControl|Delay 3.0)
          (Variables|Default|SetTutorialStep 13)
          (Widget|RemovefromParent (Variables|Default|GetSwapWeaponWidget))
          (CallFunction|ProgressTutorial Owning%20Player))))))

(event Custom|PlayerUpgradedWeapon
  (params (Owning%20Player :type Player%20Controller%20Object%20Reference))
  (if (== (Variables|Default|GetTutorialStep) 14)
    (Utilities|FlowControl|DoOnce false
      (:Completed
        (Default|CompleteStep (Variables|Default|GetUpgradeWeaponWidget))
        (Audio|SpawnSound2D "/Game/Audio/Stingers/stinger_complete.stinger_complete" 1.0 1.0 0.0 0)
        (Utilities|FlowControl|Delay 3.0)
        (Variables|Default|SetTutorialStep 15)
        (Widget|RemovefromParent (Variables|Default|GetUpgradeWeaponWidget))
        (CallFunction|ProgressTutorial Owning%20Player)))))

(event Custom|PlayerUsedJetpack
  (params (Owning%20Player :type Player%20Controller%20Object%20Reference))
  (if (== (Variables|Default|GetTutorialStep) 5)
    (Utilities|FlowControl|DoOnce false
      (:Completed
        (Default|CompleteStep (Variables|Default|GetJetpackWidget))
        (Audio|SpawnSound2D "/Game/Audio/Stingers/stinger_complete.stinger_complete" 1.0 1.0 0.0 0)
        (Utilities|FlowControl|Delay 3.0)
        (Variables|Default|SetTutorialStep 6)
        (Widget|RemovefromParent (Variables|Default|GetJetpackWidget))
        (CallFunction|ProgressTutorial Owning%20Player)))))

(event Custom|PlayerJumped
  (params (Owning%20Player :type Player%20Controller%20Object%20Reference))
  (if (== (Variables|Default|GetTutorialStep) 4)
    (Utilities|FlowControl|DoOnce false
      (:Completed
        (Default|CompleteStep (Variables|Default|GetJumpWidget))
        (Audio|SpawnSound2D "/Game/Audio/Stingers/stinger_complete.stinger_complete" 1.0 1.0 0.0 0)
        (Utilities|FlowControl|Delay 3.0)
        (Variables|Default|SetTutorialStep 5)
        (Widget|RemovefromParent (Variables|Default|GetJumpWidget))
        (CallFunction|ProgressTutorial Owning%20Player)))))

(event Custom|PlayerUsedDash
  (params (Owning%20Player :type Player%20Controller%20Object%20Reference))
  (if (== (Variables|Default|GetTutorialStep) 6)
    (Utilities|FlowControl|DoOnce false
      (:Completed
        (Default|CompleteStep (Variables|Default|GetDashWidget))
        (Audio|SpawnSound2D "/Game/Audio/Stingers/stinger_complete.stinger_complete" 1.0 1.0 0.0 0)
        (Utilities|FlowControl|Delay 3.0)
        (Variables|Default|SetTutorialStep 7)
        (Widget|RemovefromParent (Variables|Default|GetDashWidget))
        (CallFunction|ProgressTutorial Owning%20Player)))))

(event Custom|PlayerUnlockedWeapon
  (params (Owning%20Player :type Player%20Controller%20Object%20Reference))
  (if (== (Variables|Default|GetTutorialStep) 11)
    (Utilities|FlowControl|DoOnce false
      (:Completed
        (Default|CompleteStep (Variables|Default|GetUnlockWeaponWidget))
        (Audio|SpawnSound2D "/Game/Audio/Stingers/stinger_complete.stinger_complete" 1.0 1.0 0.0 0)
        (Utilities|FlowControl|Delay 3.0)
        (Variables|Default|SetTutorialStep 12)
        (Widget|RemovefromParent (Variables|Default|GetUnlockWeaponWidget))
        (CallFunction|ProgressTutorial Owning%20Player)))))

(event Custom|MovementChallengeDone
  (params (Owning%20Player :type Player%20Controller%20Object%20Reference))
  (if (== (Variables|Default|GetTutorialStep) 8)
    (Utilities|FlowControl|DoOnce false
      (:Completed
        (Default|CompleteStep (Variables|Default|GetMovementChallengeWidget))
        (Audio|SpawnSound2D "/Game/Audio/Stingers/stinger_complete.stinger_complete" 1.0 1.0 0.0 0)
        (Utilities|FlowControl|Delay 3.0)
        (Variables|Default|SetTutorialStep 9)
        (Widget|RemovefromParent (Variables|Default|GetMovementChallengeWidget))
        (CallFunction|ProgressTutorial Owning%20Player)))))

(event Custom|PlayerSprinted
  (params (OwningPlayer :type Player%20Controller%20Object%20Reference))
  (if (== (Variables|Default|GetTutorialStep) 3)
    (Utilities|FlowControl|DoOnce false
      (:Completed
        (Default|CompleteStep (Variables|Default|GetSprintWidget))
        (Audio|SpawnSound2D "/Game/Audio/Stingers/stinger_complete.stinger_complete" 1.0 1.0 0.0 0)
        (Utilities|FlowControl|Delay 3.0)
        (Variables|Default|SetTutorialStep 4)
        (Widget|RemovefromParent (Variables|Default|GetSprintWidget))
        (CallFunction|ProgressTutorial OwningPlayer)))))

(event Custom|PlayerUsedJumppad
  (params (Owning%20Player :type Player%20Controller%20Object%20Reference))
  (if (== (Variables|Default|GetTutorialStep) 7)
    (Utilities|FlowControl|DoOnce false
      (:Completed
        (Default|CompleteStep (Variables|Default|GetJumppadWidget))
        (Audio|SpawnSound2D "/Game/Audio/Stingers/stinger_complete.stinger_complete" 1.0 1.0 0.0 0)
        (Utilities|FlowControl|Delay 3.0)
        (Variables|Default|SetTutorialStep 8)
        (Widget|RemovefromParent (Variables|Default|GetJumppadWidget))
        (CallFunction|ProgressTutorial Owning%20Player)))))

(event Custom|PlayerMoved
  (params (OwningPlayer :type Player%20Controller%20Object%20Reference))
  (if (== (Variables|Default|GetTutorialStep) 0)
    (Utilities|FlowControl|DoOnce false
      (:Completed
        (Default|CompleteStep (Variables|Default|GetMoveWidget))
        (Audio|SpawnSound2D "/Game/Audio/Stingers/stinger_complete.stinger_complete" 1.0 1.0 0.0 0)
        (Utilities|FlowControl|Delay 3.0)
        (Variables|Default|SetTutorialStep 1)
        (Widget|RemovefromParent (Variables|Default|GetMoveWidget))
        (CallFunction|ProgressTutorial OwningPlayer)))))

(event Custom|PlayerKilledDrone3
  (params (Owning%20Player :type Player%20Controller%20Object%20Reference))
  (if (== (Variables|Default|GetTutorialStep) 13)
    (Utilities|FlowControl|DoOnce false
      (:Completed
        (Default|CompleteStep (Variables|Default|GetKillDrone3Widget))
        (Audio|SpawnSound2D "/Game/Audio/Stingers/stinger_complete.stinger_complete" 1.0 1.0 0.0 0)
        (Utilities|FlowControl|Delay 3.0)
        (Variables|Default|SetTutorialStep 14)
        (Widget|RemovefromParent (Variables|Default|GetKillDrone3Widget))
        (CallFunction|ProgressTutorial Owning%20Player)))))

(event Custom|PlayerKilledDrone2
  (params (Owning%20Player :type Player%20Controller%20Object%20Reference))
  (if (== (Variables|Default|GetTutorialStep) 10)
    (Utilities|FlowControl|DoOnce false
      (:Completed
        (Default|CompleteStep (Variables|Default|GetKillDrone2Widget))
        (Audio|SpawnSound2D "/Game/Audio/Stingers/stinger_complete.stinger_complete" 1.0 1.0 0.0 0)
        (Utilities|FlowControl|Delay 3.0)
        (Variables|Default|SetTutorialStep 11)
        (Widget|RemovefromParent (Variables|Default|GetKillDrone2Widget))
        (CallFunction|ProgressTutorial Owning%20Player)))))

(event Custom|PlayerUsedAltFire
  (params (Owning%20Player :type Player%20Controller%20Object%20Reference))
  (if (== (Variables|Default|GetTutorialStep) 15)
    (Utilities|FlowControl|DoOnce false
      (:Completed
        (Default|CompleteStep (Variables|Default|GetAltFireWidget))
        (Audio|SpawnSound2D "/Game/Audio/Stingers/stinger_complete.stinger_complete" 1.0 1.0 0.0 0)
        (Utilities|FlowControl|Delay 3.0)
        (Variables|Default|SetTutorialStep 16)
        (Widget|RemovefromParent (Variables|Default|GetAltFireWidget))
        (CallFunction|ProgressTutorial Owning%20Player)
        (Utilities|FlowControl|Delay 5.0)
        (Default|CompleteStep (Variables|Default|GetTutorialCompleteWidget))))))

(event Custom|PlayerFiredWeapon
  (params (Owning%20Player :type Player%20Controller%20Object%20Reference))
  (if (== (Variables|Default|GetTutorialStep) 1)
    (Utilities|FlowControl|DoOnce false
      (:Completed
        (Default|CompleteStep (Variables|Default|GetFireWeaponWidget))
        (Audio|SpawnSound2D "/Game/Audio/Stingers/stinger_complete.stinger_complete" 1.0 1.0 0.0 0)
        (Utilities|FlowControl|Delay 3.0)
        (Variables|Default|SetTutorialStep 2)
        (Widget|RemovefromParent (Variables|Default|GetFireWeaponWidget))
        (CallFunction|ProgressTutorial Owning%20Player)))))

(event Custom|PlayerSwappedWeapon
  (params (Owning%20Player :type Player%20Controller%20Object%20Reference))
  (if (== (Variables|Default|GetTutorialStep) 12)
    (Variables|Default|SetScrollSwapDone true)
    (if (and (Variables|Default|GetHotswapDone) (Variables|Default|GetScrollSwapDone))
      (Utilities|FlowControl|DoOnce false
        (:Completed
          (Default|CompleteStep (Variables|Default|GetSwapWeaponWidget))
          (Audio|SpawnSound2D "/Game/Audio/Stingers/stinger_complete.stinger_complete" 1.0 1.0 0.0 0)
          (Utilities|FlowControl|Delay 3.0)
          (Variables|Default|SetTutorialStep 13)
          (Widget|RemovefromParent (Variables|Default|GetSwapWeaponWidget))
          (CallFunction|ProgressTutorial Owning%20Player))))))

(event Custom|PlayerReloaded
  (params (Owning%20Player :type Player%20Controller%20Object%20Reference))
  (if (== (Variables|Default|GetTutorialStep) 2)
    (Utilities|FlowControl|DoOnce false
      (:Completed
        (Default|CompleteStep (Variables|Default|GetReloadWeaponWidget))
        (Audio|SpawnSound2D "/Game/Audio/Stingers/stinger_complete.stinger_complete" 1.0 1.0 0.0 0)
        (Utilities|FlowControl|Delay 3.0)
        (Variables|Default|SetTutorialStep 3)
        (Widget|RemovefromParent (Variables|Default|GetReloadWeaponWidget))
        (CallFunction|ProgressTutorial Owning%20Player)))))

(event Custom|PlayerKilledDrone
  (params (Owning%20Player :type Player%20Controller%20Object%20Reference))
  (if (== (Variables|Default|GetTutorialStep) 9)
    (Utilities|FlowControl|DoOnce false
      (:Completed
        (Default|CompleteStep (Variables|Default|GetKillDroneWidget))
        (Audio|SpawnSound2D "/Game/Audio/Stingers/stinger_complete.stinger_complete" 1.0 1.0 0.0 0)
        (Utilities|FlowControl|Delay 3.0)
        (Variables|Default|SetTutorialStep 10)
        (Widget|RemovefromParent (Variables|Default|GetKillDroneWidget))
        (CallFunction|ProgressTutorial Owning%20Player)))))

(fn SetPlayerIndex
  (bind _asbp_player_shooter_character (Utilities|Casting|CastToBP_PlayerShooterCharacter (Components|GetOwner)))
  (if (Class|ShooterCharacter|IsFirstCharacter _asbp_player_shooter_character)
    (Variables|Default|SetPlayerIndex 0)
    (else
      (Variables|Default|SetPlayerIndex 1))))