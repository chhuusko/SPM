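; Actor component that gives its owning Character a grappling hook driven by the Grapple input.
; Pressing traces forward from the owner's camera, storing the hit point; each Tick then pulls the character toward it with additive, delta-scaled LaunchCharacter calls.
; Releasing the input or reaching the max grapple timer stops the pull and starts a cooldown timer that re-enables grappling.
; Debug prints report setup, input and remaining times.
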(event EventBeginPlay
  (bind _ascharacter (Utilities|Casting|CastToCharacter (Components|GetOwner))
    (:then
      (bind _output_get (Variables|Components|SetOwningCharacter _ascharacter))
      (Variables|Default|SetCameraReference (Actor|GetComponentbyClass _output_get "/Script/Engine.CameraComponent"))
      (Development|PrintText "All setup complete!"))
    (:CastFailed
      (Development|PrintString "Failed to cast owner as character"))))

(event EventTick
  (params (DeltaSeconds :type Float%20%28single-precision%29))
  (CallFunction|GrappleWork DeltaSeconds))

(event Input|ActionEvents|InputActionGrapple
  (params (Key :type Key%20Structure :default "None"))
  (:Pressed
    (CallFunction|TriggerGrappleCheck)
    (Development|PrintString "Trigger Grapple Check done"))
  (:Released
    (CallFunction|StopGrapple)
    (Development|PrintString "Stop Grapple done")))

(fn EnableGrapple
  (Variables|Grappling|SetCanGrapple true))

(fn StopGrapple
  (if (not (Utilities|Time|IsTimerActivebyHandle (Variables|Grappling|GetCooldownTimerHandle)))
    (Variables|Grappling|SetIsGrappling false)
    (bind _returnvalue (Utilities|Time|SetTimerbyFunctionName 0 "EnableGrapple" (Variables|Grappling|GetGrappleCooldownDuration)))
    (Variables|Grappling|SetCooldownTimerHandle _returnvalue)))

(fn TriggerGrappleCheck
  (if (Variables|Grappling|GetCanGrapple)
    (CallFunction|TriggerGrapple)
    (else
      (Development|PrintString (Utilities|String|ToString(Text) (Utilities|Text|FormatText "Grapple on cooldown! Remains {Time} seconds!" (Utilities|Time|GetTimerRemainingTimebyHandle (Variables|Grappling|GetCooldownTimerHandle))))))))

(fn TriggerGrapple
  (bind _camerareference (Variables|Default|GetCameraReference))
  (bind _returnvalue (Transformation|GetWorldLocation _camerareference))
  (bind (_outhit _returnvalue_2) (Collision|LineTraceByChannel _returnvalue (+ _returnvalue (* (Math|Vector|GetForwardVector (Transformation|GetWorldRotation _camerareference)) (Variables|Grappling|GetGrappleRange))) "TraceTypeQuery4" false 0 "None"))
  (bind _output_get (Variables|Grappling|SetIsGrappling _returnvalue_2))
  (if _output_get
    (Variables|Grappling|SetCanGrapple false)
    (Variables|Grappling|SetGrappleLocation (.ImpactPoint (Collision|BreakHitResult _outhit)))))

(fn GrappleWork
  (params (DeltaSeconds :type Float%20%28single-precision%29))
  (if (Variables|Grappling|GetIsGrappling)
    (Character|LaunchCharacter (Variables|Components|GetOwningCharacter) (* DeltaSeconds (Variables|Grappling|GetGrappleStrength) (Math|Vector|Normalize (- (Variables|Grappling|GetGrappleLocation) (Transformation|GetActorLocation (Variables|Components|GetOwningCharacter)))) 10) false false)
    (if (Utilities|Time|IsTimerActivebyHandle (Variables|Grappling|GetGrappleTimerHandle))
      (Development|PrintString (Utilities|String|ToString(Text) (Utilities|Text|FormatText "Grappling! Remains {Time} seconds!" (Utilities|Time|GetTimerRemainingTimebyHandle (Variables|Grappling|GetGrappleTimerHandle)))))
      (else
        (bind _returnvalue (Utilities|Time|SetTimerbyFunctionName 0 "StopGrapple" (Variables|Grappling|GetMaxGrappleTime)))
        (Variables|Grappling|SetGrappleTimerHandle _returnvalue)))))