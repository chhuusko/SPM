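; Player shooter character that maps Enhanced Input to movement, first/third-person camera switching, weapon actions and a pause menu.
; Jumping in mid-air engages a charge-based jetpack, while dash offers timeline, lerp or single-launch variants with zeroed friction and a HUD cooldown.
; Tick drives velocity-based Niagara speed lines and cuts jetpack audio when charge runs out.
; During the tutorial, player actions and pickup milestones are reported to BPTutorialComponent.
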(event Input|EnhancedActionEvents|EnhancedInputActionIA_SwitchPerspective
  (params (ActionValue :type Boolean) (ElapsedSeconds :type Float%20%28double-precision%29) (TriggeredSeconds :type Float%20%28double-precision%29) (InputAction :type Input%20Action%20Object%20Reference :default "/Game/Inputs/IA_SwitchPerspective.IA_SwitchPerspective"))
  (:Started
    (Utilities|FlowControl|FlipFlop
      (:A
        (Components|Activation|SetActive (Variables|Default|Get1st%20Person%20Camera) false false)
        (Components|Activation|SetActive (Variables|Default|Get3rd%20Person%20Camera) true false))
      (:B
        (Components|Activation|SetActive (Variables|Default|Get3rd%20Person%20Camera) false false)
        (Components|Activation|SetActive (Variables|Default|Get1st%20Person%20Camera) true false)))))

(event Input|EnhancedActionEvents|EnhancedInputActionIA_Pause
  (params (ActionValue :type Boolean) (ElapsedSeconds :type Float%20%28double-precision%29) (TriggeredSeconds :type Float%20%28double-precision%29) (InputAction :type Input%20Action%20Object%20Reference :default "/Game/Inputs/IA_Pause.IA_Pause"))
  (bind _returnvalue (Game|GetPlayerController 0))
  (bind _returnvalue_2 (Game|GetPlayerController 0))
  (bind _returnvalue_3 (Game|GetPlayerController 1))
  ;[0.15 0.15 0.15 0.5] Pause Menu
  (:Started
    (if (not (Game|IsGamePaused))
      (bind _returnvalue_4 (UserInterface|CreateWidget "/Game/UI/WidgetBlueprints/WBP_PauseMenu.WBP_PauseMenu_C" _returnvalue))
      (bind _output_get (Variables|Default|SetPause%20Menu _returnvalue_4))
      (UserInterface|Viewport|AddtoViewport _output_get 0)
      (Input|SetInputModeUIOnly _returnvalue _output_get "DoNotLock" false)
      (Input|SetInputModeUIOnly _returnvalue_3 _output_get "DoNotLock" false)
      (Variables|/Script/Engine.PlayerController|SetbShowMouseCursor _returnvalue_2 true)
      (Game|SetGamePaused true)
      (Utilities|FlowControl|Delay 0.2)
      (Widget|SetFocus (Variables|Default|GetPause%20Menu))
      (else
        (Widget|RemovefromParent (Variables|Default|GetPause%20Menu))
        (Game|SetGamePaused false)
        (Input|SetInputModeGameOnly _returnvalue false)
        (Input|SetInputModeGameOnly _returnvalue_3 false)
        (Variables|/Script/Engine.PlayerController|SetbShowMouseCursor _returnvalue_2 false)))))

(event Input|EnhancedActionEvents|EnhancedInputActionIA_Crouch
  (params (ActionValue :type Boolean) (ElapsedSeconds :type Float%20%28double-precision%29) (TriggeredSeconds :type Float%20%28double-precision%29) (InputAction :type Input%20Action%20Object%20Reference :default "/Game/Inputs/IA_Crouch.IA_Crouch"))
  (:Started
    (Class|ShooterCharacter|SetCrouch true))
  (:Completed
    (bind _returnvalue (Class|ShooterCharacter|GetTryingtoUncrouch))
    (if (not _returnvalue)
      (Class|ShooterCharacter|SetCrouch false)
      (if (AI|Components|NavMovement|IsMovingonGround (Variables|Character|GetCharacterMovement))
        (Class|ShooterCharacter|StopSprint)))))

(event Input|EnhancedActionEvents|EnhancedInputActionIA_WeaponAbility
  (params (ActionValue :type Boolean) (ElapsedSeconds :type Float%20%28double-precision%29) (TriggeredSeconds :type Float%20%28double-precision%29) (InputAction :type Input%20Action%20Object%20Reference :default "/Game/Inputs/IA_WeaponAbility.IA_WeaponAbility"))
  (bind _returnvalue (Class|ShooterCharacter|GetGun))
  (Class|ShooterCharacter|WeaponAbility)
  (if (Math|Boolean|ANDBoolean (Variables|Default|GetIsInTutorial) (== (Variables|/Game/TutorialMap/BP_TutorialComponent.BP_TutorialComponent_C|GetTutorialStep (Variables|Default|GetBP_TutorialComponent)) 15) (Class|Gun|IsAbilityUnlocked _returnvalue) (not (== _returnvalue (Variables|Default|GetFirstAltFireUsed))))
    (Variables|Default|SetFirstAltFireUsed _returnvalue)
    (bind _result (Math|Integer|IncrementInt (Variables|Default|GetAltFiresTried))
      (:%20%20
        (if (>= _result (Variables|Default|GetAltFiresNeeded))
          (bind _asbp_shooter_player_controller (Utilities|Casting|CastToBP_ShooterPlayerController (Pawn|GetController)))
          (Default|PlayerUsedAltFire (Variables|Default|GetBP_TutorialComponent) _asbp_shooter_player_controller))))))

(event Input|EnhancedActionEvents|EnhancedInputActionIA_StopWeaponAbility
  (params (ActionValue :type Boolean) (ElapsedSeconds :type Float%20%28double-precision%29) (TriggeredSeconds :type Float%20%28double-precision%29) (InputAction :type Input%20Action%20Object%20Reference :default "/Game/Inputs/IA_StopWeaponAbility.IA_StopWeaponAbility"))
  (Class|ShooterCharacter|StopWeaponAbility))

(event Input|EnhancedActionEvents|EnhancedInputActionIA_HotSwap
  (params (ActionValue :type Boolean) (ElapsedSeconds :type Float%20%28double-precision%29) (TriggeredSeconds :type Float%20%28double-precision%29) (InputAction :type Input%20Action%20Object%20Reference :default "/Game/Inputs/WeaponSwapUnlockUpgrade/IA_HotSwap.IA_HotSwap"))
  (if (Variables|Default|GetIsInTutorial)
    (bind _asbp_shooter_player_controller (Utilities|Casting|CastToBP_ShooterPlayerController (Pawn|GetController)))
    (Default|PlayerHotswapped (Variables|Default|GetBP_TutorialComponent) _asbp_shooter_player_controller)))

(event Input|EnhancedActionEvents|EnhancedInputActionIA_SwapForward
  (params (ActionValue :type Boolean) (ElapsedSeconds :type Float%20%28double-precision%29) (TriggeredSeconds :type Float%20%28double-precision%29) (InputAction :type Input%20Action%20Object%20Reference :default "/Game/Inputs/WeaponSwapUnlockUpgrade/IA_SwapForward.IA_SwapForward"))
  (if (Variables|Default|GetIsInTutorial)
    (bind _asbp_shooter_player_controller (Utilities|Casting|CastToBP_ShooterPlayerController (Pawn|GetController)))
    (Default|PlayerSwappedWeapon (Variables|Default|GetBP_TutorialComponent) _asbp_shooter_player_controller)))

(event Input|EnhancedActionEvents|EnhancedInputActionIA_StopShooting
  (params (ActionValue :type Boolean) (ElapsedSeconds :type Float%20%28double-precision%29) (TriggeredSeconds :type Float%20%28double-precision%29) (InputAction :type Input%20Action%20Object%20Reference :default "/Game/Inputs/IA_StopShooting.IA_StopShooting"))
  (Class|ShooterCharacter|StopShooting))

(event Input|EnhancedActionEvents|EnhancedInputActionIA_Move
  (params (ActionValue :type Vector%202D%20Structure) (ElapsedSeconds :type Float%20%28double-precision%29) (TriggeredSeconds :type Float%20%28double-precision%29) (InputAction :type Input%20Action%20Object%20Reference :default "/Game/Inputs/IA_Move.IA_Move"))
  (:Triggered
    (Class|ShooterCharacter|MoveRight (.x ActionValue))
    (Class|ShooterCharacter|MoveForward (.y ActionValue))
    (Variables|Default|SetmoveX (.x ActionValue))
    (Variables|Default|SetmoveY (.y ActionValue)))
  (:Completed
    (Variables|Default|SetmoveX 0.0)
    (Variables|Default|SetmoveY 0.0)
    (Class|ShooterCharacter|StopSprint)))

(event Input|EnhancedActionEvents|EnhancedInputActionIA_CameraMovement
  (params (ActionValue :type Vector%202D%20Structure) (ElapsedSeconds :type Float%20%28double-precision%29) (TriggeredSeconds :type Float%20%28double-precision%29) (InputAction :type Input%20Action%20Object%20Reference :default "/Game/Inputs/IA_CameraMovement.IA_CameraMovement"))
  (Pawn|Input|AddControllerPitchInput (.y ActionValue))
  (if (Variables|Default|GetbCanMove)
    (Pawn|Input|AddControllerYawInput (.x ActionValue))))

(event Input|EnhancedActionEvents|EnhancedInputActionIA_Sprint
  (params (ActionValue :type Boolean) (ElapsedSeconds :type Float%20%28double-precision%29) (TriggeredSeconds :type Float%20%28double-precision%29) (InputAction :type Input%20Action%20Object%20Reference :default "/Game/Inputs/IA_Sprint.IA_Sprint"))
  (:Started
    (Class|ShooterCharacter|SetCrouch false)
    (if (AI|Components|NavMovement|IsMovingonGround (Variables|Character|GetCharacterMovement))
      (Class|ShooterCharacter|Sprint)
      (if (and (Variables|Default|GetIsInTutorial) (Variables|Default|GetIsMoving))
        (bind _asbp_shooter_player_controller (Utilities|Casting|CastToBP_ShooterPlayerController (Pawn|GetController)))
        (Default|PlayerSprinted (Variables|Default|GetBP_TutorialComponent) _asbp_shooter_player_controller))))
  (:Ongoing
    (Class|ShooterCharacter|StopReload)))

(event Input|EnhancedActionEvents|EnhancedInputActionIA_Jump
  (params (ActionValue :type Boolean) (ElapsedSeconds :type Float%20%28double-precision%29) (TriggeredSeconds :type Float%20%28double-precision%29) (InputAction :type Input%20Action%20Object%20Reference :default "/Game/Inputs/IA_Jump.IA_Jump"))
  (bind _returnvalue (Input|EnhancedActionValues|GetIA_AltDown))
  (bind _returnvalue_2 (not _returnvalue))
  (:Triggered
    (if _returnvalue_2
      (if (not (Variables|Default|GetJumped))
        (Class|ShooterCharacter|UseJetpack)
        (CallFunction|JetpackTutorial))))
  (:Started
    (if _returnvalue_2
      (CallFunction|JumpTutorial)
      (if (AI|Components|NavMovement|IsFalling (Variables|Character|GetCharacterMovement))
        (Variables|Default|SetJumped false)
        (Variables|Default|SetUsingJetpack true)
        (Class|ShooterCharacter|ConsumeJetpackChargeTap)
        (Audio|Components|Audio|FadeIn (Variables|Default|GetJetpack) 0.5 1.0 0.0 "Linear" :!class /Script/Engine.AudioComponent)
        (else
          (Character|Jump)
          (Audio|PlaySound2D "/Game/Audio/SoundCues/SC_Jump.SC_Jump" 1.0 1.0 0.0 0 0)
          (Class|ShooterCharacter|SetCrouch false)
          (Variables|Default|SetJumped true)))))
  (:Completed
    (Variables|Default|SetUsingJetpack false)
    (Audio|Components|Audio|FadeOut (Variables|Default|GetJetpack) 0.5 0.0 "Linear" :!class /Script/Engine.AudioComponent)
    (Components|Activation|SetActive (Variables|Default|GetNS_Jetpack) false false)))

(event Input|EnhancedActionEvents|EnhancedInputActionIA_Reload
  (params (ActionValue :type Boolean) (ElapsedSeconds :type Float%20%28double-precision%29) (TriggeredSeconds :type Float%20%28double-precision%29) (InputAction :type Input%20Action%20Object%20Reference :default "/Game/Inputs/IA_Reload.IA_Reload"))
  (Class|ShooterCharacter|Reload)
  (if (Variables|Default|GetIsInTutorial)
    (bind _asbp_shooter_player_controller (Utilities|Casting|CastToBP_ShooterPlayerController (Pawn|GetController)))
    (Default|PlayerReloaded (Variables|Default|GetBP_TutorialComponent) _asbp_shooter_player_controller)))

(event Input|EnhancedActionEvents|EnhancedInputActionIA_Shoot
  (params (ActionValue :type Boolean) (ElapsedSeconds :type Float%20%28double-precision%29) (TriggeredSeconds :type Float%20%28double-precision%29) (InputAction :type Input%20Action%20Object%20Reference :default "/Game/Inputs/IA_Shoot.IA_Shoot"))
  (:Started
    (Class|ShooterCharacter|Shoot)))

(event Input|EnhancedActionEvents|EnhancedInputActionIA_CameraMovementController
  (params (ActionValue :type Vector%202D%20Structure) (ElapsedSeconds :type Float%20%28double-precision%29) (TriggeredSeconds :type Float%20%28double-precision%29) (InputAction :type Input%20Action%20Object%20Reference :default "/Game/Inputs/IA_CameraMovementController.IA_CameraMovementController"))
  (Class|ShooterCharacter|LookUpRate (.y ActionValue))
  (if (Variables|Default|GetbCanMove)
    (Class|ShooterCharacter|LookRightRate (.x ActionValue))))

(event Input|EnhancedActionEvents|EnhancedInputActionIA_StopSprinting
  (params (ActionValue :type Boolean) (ElapsedSeconds :type Float%20%28double-precision%29) (TriggeredSeconds :type Float%20%28double-precision%29) (InputAction :type Input%20Action%20Object%20Reference :default "/Game/Inputs/IA_StopSprinting.IA_StopSprinting")))

(event Input|EnhancedActionEvents|EnhancedInputActionIA_Dash
  (params (ActionValue :type Boolean) (ElapsedSeconds :type Float%20%28double-precision%29) (TriggeredSeconds :type Float%20%28double-precision%29) (InputAction :type Input%20Action%20Object%20Reference :default "/Game/Inputs/IA_Dash.IA_Dash"))
  (bind _returnvalue (Pawn|GetControlRotation :!class /Script/Engine.Pawn))
  (bind _returnvalue_2 (Transformation|GetActorLocation))
  (bind _bdashzlocked (Variables|Default|GetbDashZLocked))
  (bind _charactermovement (Variables|Character|GetCharacterMovement))
  (bind _charactermovement_2 (Variables|Character|GetCharacterMovement))
  (bind _charactermovement_3 (Variables|Character|GetCharacterMovement))
  (bind _charactermovement_4 (Variables|Character|GetCharacterMovement))
  (bind _delayuntilfrictionreset (Variables|Default|GetdelayUntilFrictionReset))
  (bind _movey (Variables|Default|GetmoveY))
  (bind _returnvalue_3 (Pawn|Components|CharacterMovement|GetLastUpdateVelocity _charactermovement_4))
  (bind _returnvalue_4 (AI|Components|NavMovement|IsMovingonGround _charactermovement_2))
  (bind _returnvalue_5 (Math|Float|InRange(Float) (.pitch _returnvalue) 1.8e+02 3.6e+02))
  (bind _returnvalue_6 (and _returnvalue_5 _returnvalue_4))
  (bind _returnvalue_7 (Math|Boolean|NORBoolean _bdashzlocked _returnvalue_6))
  (bind _returnvalue_8 (* (.pitch _returnvalue) _returnvalue_7))
  (bind _returnvalue_9 (Math|Vector|GetForwardVector (Math|Rotator|MakeRotator 0.0 _returnvalue_8 (.yaw _returnvalue))))
  (bind _returnvalue_10 (Math|Vector|Normalize _returnvalue_9))
  (:Started
    (CallFunction|XYinRange (Variables|Default|GetmoveX) (Variables|Default|GetmoveY))
    ;[0.15 0.15 0.15 0.5] Start of Dash
    (if (and true (Variables|Default|GetbCanDash))
      (CallFunction|DashTutorial)
      (Variables|Default|SetbCanDash false)
      (Variables|Default|SetDashPitchRotation (.pitch _returnvalue))
      (Variables|Default|SetFrictionToReset (Variables|/Script/Engine.CharacterMovementComponent|GetGroundFriction _charactermovement))
      (Variables|/Script/Engine.CharacterMovementComponent|SetGroundFriction _charactermovement 0.0)
      (CallFunction|SetDashVFX true)
      (Audio|PlaySoundatLocation "/Game/Audio/SoundCues/SC_Dash.SC_Dash" (Transformation|GetActorLocation) "0, 0, 0" 1.0 1.0 0.0 0 0 0 0)
      (if (Variables|Default|GetTimeline%20Dash)
        (if (or (!= _movey 0.0) (!= (Variables|Default|GetmoveX) 0.0))
          (Variables|Default|SetDashDirection (Math|Vector|Normalize (Math|Vector|MakeVector (.x _returnvalue_3) (.y _returnvalue_3) (* (* (+ (* (Math|Float|InRange(Float) (Variables|Default|GetDashPitchRotation) 2.7e+02 3.6e+02) (- 3.6e+02 (Variables|Default|GetDashPitchRotation)) -1.0) (* (not (Math|Float|InRange(Float) (Variables|Default|GetDashPitchRotation) 2.7e+02 3.6e+02)) (Variables|Default|GetDashPitchRotation))) (Math|Vector|VectorLength (Math|Vector|MakeVector (.x _returnvalue_3) (.y _returnvalue_3) (.z _returnvalue_3))) 0.02) _movey))))
          (bind _alpha (Timeline|Dash%20Timeline PlayFromStart)
            (:Update
              (Character|LaunchCharacter (* (Variables|Default|GetDashDirection) (* (Variables|Default|GetdashDistance) _alpha (+ (- (* (- 3.6e+02 (Variables|Default|GetDashPitchRotation)) 2.5 (AI|Components|NavMovement|IsMovingonGround (Variables|Character|GetCharacterMovement)) (Math|Float|InRange(Float) (Variables|Default|GetDashPitchRotation) 1.8e+02 3.6e+02)) (* (Variables|Default|GetDashPitchRotation) (Math|Float|InRange(Float) (Variables|Default|GetDashPitchRotation) 0.0 9e+01) 0.25)) 5e+01))) true true))
            (:Finished
              (bind _asshooter_player_controller (Utilities|Casting|CastToShooterPlayerController (Pawn|GetController) :!label _label))
              (Class|HUDWidget|StartDashTimer (Variables|/Script/SPM.ShooterPlayerController|GetHUDWidget _asshooter_player_controller) (+ (Variables|Default|GetdashCooldownSeconds) (Variables|Default|GetdelayUntilFrictionReset)))
              (Utilities|FlowControl|Delay _delayuntilfrictionreset)
              (Variables|/Script/Engine.CharacterMovementComponent|SetGroundFriction _charactermovement_3 (Variables|Default|GetFrictionToReset))
              (CallFunction|SetDashVFX false)
              (Utilities|FlowControl|Delay (- (Variables|Default|GetdashCooldownSeconds) _delayuntilfrictionreset))
              (if (Variables|Default|GetbLerpDash)
                _
                (else
                  (Variables|/Script/Engine.MovementComponent|SetVelocity _charactermovement_3 (* (Transformation|GetVelocity) (Variables|Default|GetDashSmoothing)))))
              ;[0.15 0.15 0.15 0.5] Dash CD Over
              (Variables|Default|SetbCanDash true)))
          (else
            (Variables|Default|SetDashDirection (Math|Vector|Normalize (Math|Vector|GetForwardVector (Pawn|GetControlRotation :!class /Script/Engine.Pawn))))
            (Timeline|Dash%20Timeline PlayFromStart)))
        (elif (Variables|Default|GetbLerpDash)
          ;[0.15 0.15 0.15 0.5] Lerp Dash
          (bind _alpha_2 (Timeline|Timeline PlayFromStart)
            (:Update
              (Transformation|SetActorLocation (Math|Vector|Lerp(Vector) _returnvalue_2 (+ (* _returnvalue_10 (Variables|Default|GetdashDistance)) _returnvalue_2) _alpha_2) true false)
              (goto _label)))
          (else
            ;[0.15 0.15 0.15 0.5] Launch Dash
            (Character|LaunchCharacter (* _returnvalue_10 (* (Variables|Default|GetdashDistance) 5e+01)) true true)
            (goto _label)))))))

(event EventBeginPlay
  (|CallParentFunction))

(event Collision|EventActorBeginOverlap
  (params (OtherActor :type Actor%20Object%20Reference))
  (|CallParentFunction OtherActor) ; This node is disabled and will not be called.\nDrag off pins to build functionality.
)

(event EventTick
  (params (DeltaSeconds :type Float%20%28single-precision%29))
  (bind _charactermovement (Variables|Character|GetCharacterMovement))
  (bind _returnvalue (Pawn|Components|CharacterMovement|GetLastUpdateVelocity _charactermovement))
  (bind _returnvalue_2 (Math|Vector|VectorLength _returnvalue))
  (|CallParentFunction DeltaSeconds)
  (Class|ShooterCharacter|GetTryingtoUncrouch)
  (if (> _returnvalue_2 (Variables|Default|GetSpeedLineVelocity))
    (Components|Activation|SetActive (Variables|Default|GetNS_Dash) true false)
    (Effects|Components|ParticleSystem|SetFloatParameter (Variables|Default|GetNS_Dash) "VelocitySpawnRate" (* _returnvalue_2 0.2))
    (else
      (Components|Activation|SetActive (Variables|Default|GetNS_Dash) false false)))
  (CallFunction|JetpackSound))

(event EventOnPlayerPickup
  (params (PlayerCharacter :type Shooter%20Character%20Object%20Reference))
  (bind _bp_tutorialcomponent (Variables|Default|GetBP_TutorialComponent))
  (if (Variables|Default|GetIsInTutorial)
    (bind _asbp_perspective_shooter_character (Utilities|Casting|CastToBP_PerspectiveShooterCharacter PlayerCharacter))
    (bind _asbp_shooter_player_controller (Utilities|Casting|CastToBP_ShooterPlayerController (Pawn|GetController PlayerCharacter)))
    (Default|PlayerFiredWeapon _bp_tutorialcomponent _asbp_shooter_player_controller)
    (bind _returnvalue (Class|Resources|GetResourceAmount (Variables|/Game/CharacterBPS/BP_PerspectiveShooterCharacter.BP_PerspectiveShooterCharacter_C|GetResources _asbp_perspective_shooter_character)))
    (if (>= _returnvalue 4)
      (Default|PlayerKilledDrone3 _bp_tutorialcomponent _asbp_shooter_player_controller)
      (elif (>= _returnvalue 2)
        (Default|PlayerKilledDrone2 _bp_tutorialcomponent _asbp_shooter_player_controller)))))

(event EventOnWeaponUnlocked
  (params (WeaponType :type EWeaponType%20Enum :default "Pistol"))
  (if (Variables|Default|GetIsInTutorial)
    (bind _asbp_shooter_player_controller (Utilities|Casting|CastToBP_ShooterPlayerController (Pawn|GetController)))
    (Default|PlayerUnlockedWeapon (Variables|Default|GetBP_TutorialComponent) _asbp_shooter_player_controller)))

(event EventOnWeaponUpgraded
  (if (Variables|Default|GetIsInTutorial)
    (bind _asbp_shooter_player_controller (Utilities|Casting|CastToBP_ShooterPlayerController (Pawn|GetController)))
    (Default|PlayerUpgradedWeapon (Variables|Default|GetBP_TutorialComponent) _asbp_shooter_player_controller)))

(event EventOnLanded
  (params (Hit :type Hit%20Result%20Structure%20%28by%20ref%29))
  (if (Variables|Default|GetbCrouching)
    (Class|ShooterCharacter|StopSprint)))

(event Input|AxisEvents|InputAxisMoveForward
  (params (AxisValue :type Float%20%28single-precision%29))
  ;[0.15 0.15 0.15 0.5] Tutorial
  (if (Variables|Default|GetIsInTutorial)
    (if (== AxisValue 0.0)
      (Variables|Default|SetIsMoving false)
      (else
        (bind _asbp_shooter_player_controller (Utilities|Casting|CastToBP_ShooterPlayerController (Pawn|GetController)))
        (Default|PlayerMoved (Variables|Default|GetBP_TutorialComponent) _asbp_shooter_player_controller)
        (Variables|Default|SetIsMoving true)))))

(event Input|AxisEvents|InputAxisMoveRight
  (params (AxisValue :type Float%20%28single-precision%29))
  ;[0.15 0.15 0.15 0.5] Tutorial
  (if (Variables|Default|GetIsInTutorial)
    (if (== AxisValue 0.0)
      (Variables|Default|SetIsMoving false)
      (else
        (bind _asbp_shooter_player_controller (Utilities|Casting|CastToBP_ShooterPlayerController (Pawn|GetController)))
        (Default|PlayerMoved (Variables|Default|GetBP_TutorialComponent) _asbp_shooter_player_controller)
        (Variables|Default|SetIsMoving true)))))

(fn ConstructionScript
  (|CallParentFunction))

(fn XYinRange
  (params (X :type Float%20%28double-precision%29) (Y :type Float%20%28double-precision%29))
  (return (not (and (Math|Float|InRange(Float) X -0.1 0.1) (Math|Float|InRange(Float) Y -0.1 0.1)))))

(fn DashTutorial
  (if (Variables|Default|GetIsInTutorial)
    (bind _asbp_shooter_player_controller (Utilities|Casting|CastToBP_ShooterPlayerController (Pawn|GetController)))
    (Default|PlayerUsedDash (Variables|Default|GetBP_TutorialComponent) _asbp_shooter_player_controller)))

(fn JumpTutorial
  (if (Variables|Default|GetIsInTutorial)
    (bind _asbp_shooter_player_controller (Utilities|Casting|CastToBP_ShooterPlayerController (Pawn|GetController)))
    (Default|PlayerJumped (Variables|Default|GetBP_TutorialComponent) _asbp_shooter_player_controller)))

(fn JetpackTutorial
  (if (Variables|Default|GetIsInTutorial)
    (bind _asbp_shooter_player_controller (Utilities|Casting|CastToBP_ShooterPlayerController (Pawn|GetController)))
    (Default|PlayerUsedJetpack (Variables|Default|GetBP_TutorialComponent) _asbp_shooter_player_controller)))

(fn JetpackSound
  (if (Variables|Default|GetUsingJetpack)
    (bind _returnvalue (Class|ShooterCharacter|GetJetpackCharge))
    (if (== _returnvalue 0.0)
      (Audio|Components|Audio|FadeOut (Variables|Default|GetJetpack) 0.5 0.0 "Linear" :!class /Script/Engine.AudioComponent))))

(fn SprintifMovingforSomeTime
  (params (A :type Float%20%28double-precision%29))
  (bind _output_get (Variables|Default|SetMoveTime (+ A (Variables|Default|GetMoveTime))))
  (if (and (>= _output_get 0.5) (not (Variables|Default|GetIsSprinting)))
    (Class|ShooterCharacter|Sprint)
    (Variables|Default|SetIsSprinting true)))

(fn StopSprintingifSprinting
  (Variables|Default|SetMoveTime 0.0)
  (if (Variables|Default|GetIsSprinting)
    (Class|ShooterCharacter|StopSprint)
    (Variables|Default|SetIsSprinting false)))

(fn AutoSprint
  (params (A :type Float%20%28double-precision%29))
  (bind _output_get (Variables|Default|SetIsMoving (>= (Math|Vector|VectorLength (Transformation|GetVelocity)) 1e+01)))
  (if _output_get
    (CallFunction|SprintifMovingforSomeTime A)
    (else
      (CallFunction|StopSprintingifSprinting))))

(fn SetDashVFX
  (params (Active :type Boolean)))