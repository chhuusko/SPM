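; Game mode Blueprint that binds two local players to the platform users stored in the ShooterGameInstance.
; One tick after BeginPlay, it calls SetPlayer for player indices 0 and 1.
; SetPlayer selects the matching platform ID from the game instance and, if that ID is valid, assigns it to that index's player controller.
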(event EventBeginPlay
  (Utilities|FlowControl|DelayUntilNextTick)
  (CallFunction|SetPlayer)
  (CallFunction|SetPlayer 1))

(fn ConstructionScript)

(fn SetPlayer
  (params (PlayerIndex :type Integer))
  (bind _asshooter_game_instance (Utilities|Casting|CastToShooterGameInstance (Game|GetGameInstance)))
  (if (Class|InputDeviceLibrary|IsValidPlatformId (Utilities|Select :Index PlayerIndex :Option%200 (Class|ShooterGameInstance|GetPlayer1PlatformId _asshooter_game_instance) :Option%201 (Class|ShooterGameInstance|GetPlayer2PlatformId _asshooter_game_instance)))
    (Class|GameplayStatics|SetPlayerPlatformUserId (Game|GetPlayerController PlayerIndex) (Utilities|Select :Index PlayerIndex :Option%200 (Class|ShooterGameInstance|GetPlayer1PlatformId _asshooter_game_instance) :Option%201 (Class|ShooterGameInstance|GetPlayer2PlatformId _asshooter_game_instance)))))